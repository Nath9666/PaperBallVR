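; BP_DebugPawn is a debug pawn that throws BP_Can actors in the direction of the control rotation.
; BeginPlay adds the IMC_Debug mapping context, and IA_Throw spawns a can offset forward from the pawn by PositionCan.
; The can's static mesh gets a ThrowForce impulse as a velocity change, so mass is ignored.
; A PrintLog helper reports throws and force, gated by the Debug flag.
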(event `self.ReceiveBeginPlay`
  (`EnhancedInputSubsystemInterface.AddMappingContext` (pcsubsystem `EnhancedInputLocalPlayerSubsystem` (`GameplayStatics.GetPlayerController` 0)) "/Game/XRFramework/Input/IMC_Debug.IMC_Debug" 1 (struct)))

(event `EnhancedInput|/Game/XRFramework/Input/Actions/IA_Throw`
  (params (ActionValue :type Boolean) (ElapsedSeconds :type "Float (double-precision)") (TriggeredSeconds :type "Float (double-precision)") (InputAction :type "InputAction Object Reference" :default "/Game/XRFramework/Input/Actions/IA_Throw.IA_Throw"))
  (bind _returnvalue (`self.GetControlRotation`))
  (bind _throwforce (`self.ThrowForce`))
  (:`Started`
    (`self.Print_log` (`self.Debug`) "Canette lancé" "Can")
    (bind _returnvalue_2 (`|SpawnActorFromClass` "/Game/UNIVERSITY_CLASSROOM/Blueprints/BP_Can.BP_Can_C" (`KismetMathLibrary.MakeTransform` (+ (`self.K2_GetActorLocation`) (* (`KismetMathLibrary.GetForwardVector` _returnvalue) (`self.Position Can`))) _returnvalue) "AlwaysSpawn" "MultiplyWithRoot" null null))
    (`PrimitiveComponent.AddImpulse` (`/Game/UNIVERSITY_CLASSROOM/Blueprints/BP_Can.StaticMesh` _returnvalue_2) (* (`KismetMathLibrary.GetForwardVector` (`self.GetControlRotation`)) _throwforce) "None" true)
    (`self.Print_log` (`self.Debug`) (`KismetStringLibrary.Conv_DoubleToString` _throwforce) "Power")))

(fn `Print_log`
  (params (Debut :type Boolean) (Print :type String) (Key :type Name))
  (`KismetSystemLibrary.PrintString` Print Debut Debut (struct :`G` 0.66 :`B` 1.0 :`A` 1.0) 2.0 Key))

(fn `UserConstructionScript`)