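; BP_WallClock is a classroom wall clock actor that displays a time value and a score on text render components.
; UpdateDisplay splits the seconds it receives into minutes and seconds, without zero-padding, and sets both texts.
; The time text turns red at 15 seconds or fewer, with no reset to another color.
; The event graph and construction script are empty, so the clock keeps no time of its own.
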(fn `UpdateDisplay`
  (params (Seconds :type Integer) (Score :type Integer))
  (locals (Minutes :type Integer) (Seondes :type Integer))
  (bind _output_get (set `local.Minutes` (/ Seconds 60)))
  (bind _output_get_2 (set `local.Seondes` (mod Seconds 60)))
  (`TextRenderComponent.K2_SetText` (`self.TimeText`) (`KismetTextLibrary.Conv_StringToText` (`KismetStringLibrary.BuildString_Int` (`KismetStringLibrary.Conv_IntToString` _output_get) ":" _output_get_2)))
  (`TextRenderComponent.K2_SetText` (`self.ScoreText`) (`KismetTextLibrary.Conv_StringToText` (`KismetStringLibrary.BuildString_Int` "Score : " "" Score)))
  (if (<= Seconds 15)
    (`TextRenderComponent.SetTextRenderColor` (`self.TimeText`) (`KismetMathLibrary.Conv_LinearColorToColor` (struct :`R` 1.0 :`A` 1.0)))))

(fn `UserConstructionScript`)