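; BP_LevelManager runs level progression for a bin-scoring minigame, setting the bin's mode for each level.
; On BeginPlay it finds BP_Bin, binds to its scored event and applies the current level.
; Each score raises total and per-level counters, and reaching a per-level threshold advances the level and switches the bin mode.
; Score and mode appear via debug prints, and levels past the third use an effectively unreachable threshold.
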(event `self.ReceiveBeginPlay`
  (bind _returnvalue (`GameplayStatics.GetActorOfClass` "/Game/UNIVERSITY_CLASSROOM/Blueprints/BP_Bin.BP_Bin_C"))
  (set `self.Bin` _returnvalue)
  (add `/Game/UNIVERSITY_CLASSROOM/Blueprints/BP_Bin.OnScored` (`self.Bin`) (delegate `HandleScored`))
  (`self.ApplyLevel`))

(event `HandleScored`
  (`self.AddScore`))

(fn `AddScore`
  (bind _score (`self.Score`))
  (`/Engine/EditorBlueprintResources/StandardMacros.IncrementInt` _score
    (:`  `
      (`/Engine/EditorBlueprintResources/StandardMacros.IncrementInt` (`self.ScoreInLevel`)
        (:`  `
          (`KismetSystemLibrary.PrintString` (`KismetStringLibrary.BuildString_Int` "Score " "" _score) true true (struct :`G` 0.66 :`B` 1.0 :`A` 1.0) 2.0 "Score")
          (if (>= (`self.ScoreInLevel`) (`self.GetRequiredScore`))
            (`self.NextLevel`)))))))

(fn `ApplyLevel`
  (locals (CurentMode :type "/Game/UNIVERSITY_CLASSROOM/Blueprints/E_BinMode Enum"))
  (bind _bin (`self.Bin`))
  (switch `int` (`self.CurentLevel`)
    (:`0`
      (bind _output_get (set `local.CurentMode` "NewEnumerator0"))
      (`/Game/UNIVERSITY_CLASSROOM/Blueprints/BP_Bin.SetMode` _bin _output_get))
    (:`1`
      (bind _output_get_2 (set `local.CurentMode` "NewEnumerator1" :!label _label))
      (`/Game/UNIVERSITY_CLASSROOM/Blueprints/BP_Bin.SetMode` _bin _output_get_2))
    (:`2`
      (bind _output_get_3 (set `local.CurentMode` "NewEnumerator2"))
      (`/Game/UNIVERSITY_CLASSROOM/Blueprints/BP_Bin.SetMode` _bin _output_get_3))
    (:`3`
      (goto _label)))
  (`KismetSystemLibrary.PrintString` (`|GetEnumeratorNameAsString` (`local.CurentMode`)) true true (struct :`G` 1.0 :`B` 0.121439 :`A` 1.0) 3.0 "Bin Mode"))

(fn `GetRequiredScore`
  (returns (RequiredScore :type Integer))
  (switch `int` (`self.CurentLevel`)
    (:`Default`
      (return 999))
    (:`0`
      (return 2))
    (:`1`
      (return 3))
    (:`2`
      (return 5))))

(fn `NextLevel`
  (`/Engine/EditorBlueprintResources/StandardMacros.IncrementInt` (`self.CurentLevel`)
    (:`  `
      (set `self.ScoreInLevel` 0)
      (`self.ApplyLevel`))))

(fn `UserConstructionScript`)