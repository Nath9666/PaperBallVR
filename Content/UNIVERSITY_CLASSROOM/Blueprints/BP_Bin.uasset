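; BP_Bin is a bin actor that scores BP_Can actors that land in its ScoreZone.
; On overlap, it checks and sets the can's Scored flag to avoid double counting, increments its own Score, then destroys the can.
; The running score is shown through a PrintLog helper that wraps PrintString with a debug toggle and a message key.
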(event `self.ScoreZone.OnComponentBeginOverlap`
  (params (OverlappedComponent :type "PrimitiveComponent Object Reference") (OtherActor :type "Actor Object Reference") (OtherComp :type "PrimitiveComponent Object Reference") (OtherBodyIndex :type Integer) (bFromSweep :type Boolean) (SweepResult :type "HitResult Structure (by ref)"))
  (bind _score (`self.Score`))
  (bind _asbp_can (cast `/Game/UNIVERSITY_CLASSROOM/Blueprints/BP_Can` OtherActor))
  (if (not (`/Game/UNIVERSITY_CLASSROOM/Blueprints/BP_Can.bScored` _asbp_can))
    (set `/Game/UNIVERSITY_CLASSROOM/Blueprints/BP_Can.bScored` true _asbp_can)
    (`/Engine/EditorBlueprintResources/StandardMacros.IncrementInt` _score
      (:`  `
        (`self.Print_log` true (`KismetStringLibrary.Conv_IntToString` _score) "Score")
        (`self.K2_DestroyActor` _asbp_can)))))

(fn `Print_log`
  (params (Debut :type Boolean) (Print :type String) (Key :type Name))
  (`KismetSystemLibrary.PrintString` Print Debut Debut (struct :`G` 0.66 :`B` 1.0 :`A` 1.0) 2.0 Key))

(fn `UserConstructionScript`)